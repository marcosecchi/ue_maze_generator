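; BP_TileBase is a base tile with four walls whose open or closed state follows a tile ID.
; InitTile clamps the ID between -1 and 15, then Init shows it on a text render and updates each cardinal wall.
; HasDoor resolves each direction's opening from the ID, and CheckWall swaps that side's static mesh to the open or closed variant.
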(event EventBeginPlay)

(event EventInitTile
  (params (TileId :type Integer))
  (Variables|TileSettings|SetTileId (Math|Integer|Clamp(Integer) TileId -1 15))
  (CallFunction|Init))

(fn ConstructionScript)

(fn Init
  (Utilities|FlowControl|Sequence
    (:then_0
      (Rendering|Components|TextRender|SetText (Variables|Default|GetTextRender) (Utilities|Text|ToText(Integer) (Variables|TileSettings|GetTileId))))
    (:then_1
      (CallFunction|CheckWall (Variables|Default|GetStaticMesh_N) (CallFunction|HasDoor "North" (Variables|TileSettings|GetTileId))))
    (:then_2
      (CallFunction|CheckWall (Variables|Default|GetStaticMesh_S) (CallFunction|HasDoor "South" (Variables|TileSettings|GetTileId))))
    (:then_3
      (CallFunction|CheckWall (Variables|Default|GetStaticMesh_E) (CallFunction|HasDoor "East" (Variables|TileSettings|GetTileId))))
    (:then_4
      (CallFunction|CheckWall (Variables|Default|GetStaticMesh_W) (CallFunction|HasDoor "West" (Variables|TileSettings|GetTileId))))))

(fn CheckWall
  (params (MeshComponent :type Static%20Mesh%20Component%20Object%20Reference) (IsOpen :type Boolean))
  (if IsOpen
    (Components|StaticMesh|SetStaticMesh MeshComponent (Variables|Default|GetOpenWallMesh))
    (return)
    (else
      (Components|StaticMesh|SetStaticMesh MeshComponent (Variables|Default|GetClosedWallMesh))
      (return))))