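; Tile generator actor that builds a maze level from spawned tile actors when play begins.
; GenerateMaze returns a map of grid coordinates to tile data, driven by size, maze type, selection percentage and random tile removal settings.
; Each coordinate spawns a TileClass actor spaced from the generator's location, with grid X running along negative world X.
; Each tile then receives its map value through InitTileMessage.
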(event EventBeginPlay
  (bind _returnvalue (Transformation|GetActorLocation))
  (bind _spacing (Variables|Default|GetSpacing))
  (bind _returnvalue_2 (Class|MazeGeneratorFunctionLibrary|GenerateMaze (Variables|Default|GetNumRows) (Variables|Default|GetNumColumns) (Variables|Default|GetMaze%20Type) (Variables|Default|GetType%20Selection%20Percentage) (Variables|Default|GetNum%20Randomly%20Removed%20Tiles)))
  (bind _output_get (Variables|Default|SetMap _returnvalue_2))
  (bind _keys (Utilities|Map|Keys _output_get))
  (for _array_element _keys
    (bind _returnvalue_3 (Game|SpawnActorfromClass (Variables|Default|GetTileClass) (Math|Transform|MakeTransform (Math|Vector|MakeVector (+ (* (.X (Utilities|Struct|BreakIntVector _array_element)) _spacing -1.0) (.x _returnvalue)) (+ (* (.Y (Utilities|Struct|BreakIntVector _array_element)) _spacing) (.y _returnvalue)) 0.0) "0, 0, 0" "1.000000,1.000000,1.000000") "Undefined" "MultiplyWithRoot" 0 0))
    (Class|WangTileInterface|InitTile(Message) _returnvalue_3 (.Value (Utilities|Map|Find (Variables|Default|GetMap) _array_element)))))

(fn ConstructionScript)