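; Utility function library that generates Wang tile grids as maps of row/column coordinates to tile IDs, with doors stored as a four-bit N/E/S/W mask.
; GenerateGrid dispatches to empty (-1), random, checkerboard or labyrinth generators.
; Checkerboard randomizes alternate tiles, derives the rest from neighboring doors, and its closed variant strips border doors.
; Perfect Labyrinth is unfinished, returning an empty grid; GenerateRandomTile and ProcessPerfectLabirynthTile are stubs.
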(fn HasDoor
  (params (Direction :type DoorDirection%20Enum :default "NewEnumerator0") (TileId :type Integer))
  ;[1 1 1] Checks if there is a door in the requested direction through a bitwise operation
  (switch Utilities|FlowControl|Switch|SwitchonDoorDirection Direction
    (:NewEnumerator0
      (LocalVariables|SetMask 1))
    (:NewEnumerator1
      (LocalVariables|SetMask 2))
    (:NewEnumerator2
      (LocalVariables|SetMask 4))
    (:NewEnumerator3
      (LocalVariables|SetMask 8)))
  (return (== (Class|KismetMathLibrary|AndIntInt TileId (LocalVariables|GetMask)) (LocalVariables|GetMask))))

(fn GenerateGrid
  (params (GenerationType :type TileGeneration_Type%20Enum :default "NewEnumerator3") (NumRows :type Integer) (NumColumns :type Integer))
  (switch Utilities|FlowControl|Switch|SwitchonTileGeneration_Type GenerationType
    (:NewEnumerator3
      (bind _result (CallFunction|GenerateEmpty NumRows NumColumns))
      (return _result))
    (:NewEnumerator0
      (bind _result_2 (CallFunction|GenerateRandom NumRows NumColumns))
      (return _result_2))
    (:NewEnumerator4
      (bind _result_3 (CallFunction|GenerateCheckerboard NumRows NumColumns false))
      (return _result_3))
    (:NewEnumerator1
      (bind _result_4 (CallFunction|GenerateCheckerboard NumRows NumColumns true))
      (return _result_4))
    (:NewEnumerator2
      (bind _result_5 (CallFunction|GeneratePerfectLabyrinth NumRows NumColumns))
      (return _result_5))))

(fn GenerateEmpty
  (params (NumRows :type Integer) (NumColumns :type Integer))
  ;[1 1 1] Generates and empty grid with tiles set to -1
  (for _index (range 0 (- NumRows 1))
    (for _index_2 (range 0 (- NumColumns 1))
      (Utilities|Map|Add (LocalVariables|GetL_Map) (Utilities|Struct|MakeIntVector _index _index_2) -1)))
  (return (LocalVariables|GetL_Map)))

(fn GenerateRandom
  (params (NumRows :type Integer) (NumColumns :type Integer))
  ;[1 1 1] Generates a totally random grid with no door checks
  (bind _result (CallFunction|GenerateEmpty NumRows NumColumns))
  (bind _output_get (LocalVariables|SetL_Map _result))
  (bind _keys (Utilities|Map|Keys _output_get))
  (for _array_element _keys
    (LocalVariables|SetL_TileCoord _array_element)
    (Utilities|Map|Add (LocalVariables|GetL_Map) (LocalVariables|GetL_TileCoord) (Math|Random|RandomIntegerinRange 0 15)))
  (return (LocalVariables|GetL_Map)))

(fn GenerateCheckerboard
  (params (NumRows :type Integer) (NumColumns :type Integer) (IsClosed :type Boolean))
  (bind _result (CallFunction|GenerateEmpty NumRows NumColumns))
  (bind _output_get (LocalVariables|SetL_Map _result))
  (bind _keys (Utilities|Map|Keys _output_get))
  (LocalVariables|SetL_Keys _keys)
  (Utilities|FlowControl|Sequence
    (:then_0
      ;[1 1 1] Generate random tiles
      (for _array_element (LocalVariables|GetL_Keys)
        (bind _output_get_2 (LocalVariables|SetL_TileCoord _array_element))
        (if (== (Math|Integer|%(Integer) (.x _output_get_2) 2) 0)
          (if (== (Math|Integer|%(Integer) (.y (LocalVariables|GetL_TileCoord)) 2) 0)
            (Utilities|Map|Add (LocalVariables|GetL_Map) (LocalVariables|GetL_TileCoord) (Math|Random|RandomIntegerinRange 0 15) :!label _label))
          (elif (not (== (Math|Integer|%(Integer) (.y (LocalVariables|GetL_TileCoord)) 2) 0))
            (goto _label)))))
    (:then_1
      ;[1 1 1] Get non-generated tiles
      (for _array_element_2 (LocalVariables|GetL_Keys)
        (bind _output_get_3 (LocalVariables|SetL_TileCoord _array_element_2))
        (if (== (Math|Integer|%(Integer) (.x _output_get_3) 2) 0)
          (if (!= (Math|Integer|%(Integer) (.y (LocalVariables|GetL_TileCoord)) 2) 0)
            (LocalVariables|SetL_TileId 0 :!label _label_2)
            (Utilities|FlowControl|Sequence
              (:then_0
                ;[1 1 1] Check if has door: North
                (if (and (.ReturnValue (Utilities|Map|Find (LocalVariables|GetL_Map) (Utilities|Struct|MakeIntVector (+ (.x (LocalVariables|GetL_TileCoord)) -1) (.y (LocalVariables|GetL_TileCoord))))) (CallFunction|HasDoor "NewEnumerator2" (.Value (Utilities|Map|Find (LocalVariables|GetL_Map) (Utilities|Struct|MakeIntVector (+ (.x (LocalVariables|GetL_TileCoord)) -1) (.y (LocalVariables|GetL_TileCoord)))))))
                  (bind _result_2 (CallFunction|AddDoor "NewEnumerator0" (LocalVariables|GetL_TileId)))
                  (LocalVariables|SetL_TileId _result_2)))
              (:then_1
                ;[1 1 1] Check if has door: South
                (if (and (.ReturnValue (Utilities|Map|Find (LocalVariables|GetL_Map) (Utilities|Struct|MakeIntVector (+ (.x (LocalVariables|GetL_TileCoord)) 1) (.y (LocalVariables|GetL_TileCoord))))) (CallFunction|HasDoor "NewEnumerator0" (.Value (Utilities|Map|Find (LocalVariables|GetL_Map) (Utilities|Struct|MakeIntVector (+ (.x (LocalVariables|GetL_TileCoord)) 1) (.y (LocalVariables|GetL_TileCoord)))))))
                  (bind _result_3 (CallFunction|AddDoor "NewEnumerator2" (LocalVariables|GetL_TileId)))
                  (LocalVariables|SetL_TileId _result_3)))
              (:then_2
                ;[1 1 1] Check if has door: East
                (if (and (.ReturnValue (Utilities|Map|Find (LocalVariables|GetL_Map) (Utilities|Struct|MakeIntVector (.x (LocalVariables|GetL_TileCoord)) (+ (.y (LocalVariables|GetL_TileCoord)) 1)))) (CallFunction|HasDoor "NewEnumerator3" (.Value (Utilities|Map|Find (LocalVariables|GetL_Map) (Utilities|Struct|MakeIntVector (.x (LocalVariables|GetL_TileCoord)) (+ (.y (LocalVariables|GetL_TileCoord)) 1))))))
                  (bind _result_4 (CallFunction|AddDoor "NewEnumerator1" (LocalVariables|GetL_TileId)))
                  (LocalVariables|SetL_TileId _result_4)))
              (:then_3
                ;[1 1 1] Check if has door: East
                (if (and (.ReturnValue (Utilities|Map|Find (LocalVariables|GetL_Map) (Utilities|Struct|MakeIntVector (.x (LocalVariables|GetL_TileCoord)) (+ (.y (LocalVariables|GetL_TileCoord)) -1)))) (CallFunction|HasDoor "NewEnumerator1" (.Value (Utilities|Map|Find (LocalVariables|GetL_Map) (Utilities|Struct|MakeIntVector (.x (LocalVariables|GetL_TileCoord)) (+ (.y (LocalVariables|GetL_TileCoord)) -1))))))
                  (bind _result_5 (CallFunction|AddDoor "NewEnumerator3" (LocalVariables|GetL_TileId)))
                  (LocalVariables|SetL_TileId _result_5)))
              (:then_4
                ;[1 1 1] Add tile to map
                (Utilities|Map|Add (LocalVariables|GetL_Map) (LocalVariables|GetL_TileCoord) (LocalVariables|GetL_TileId)))))
          (elif (not (!= (Math|Integer|%(Integer) (.y (LocalVariables|GetL_TileCoord)) 2) 0))
            (goto _label_2)))))
    (:then_2
      (if IsClosed
        ;[1 1 1] Return final map with closed external doors
        (bind _result_6 (CallFunction|RemoveExternalDoors (LocalVariables|GetL_Map)))
        (return _result_6)
        (else
          ;[1 1 1] Return final map
          (return (LocalVariables|GetL_Map)))))))

(fn GeneratePerfectLabyrinth
  (params (NumRows :type Integer) (NumColumns :type Integer))
  (bind _result (CallFunction|GenerateEmpty NumRows NumColumns))
  (LocalVariables|SetL_Map _result)
  (Utilities|FlowControl|Sequence
    (:then_0
      ;[1 1 1] init
      (bind _result_2 (CallFunction|GetGridSize (LocalVariables|GetL_Map)))
      (bind _output_get (LocalVariables|SetL_GridSize _result_2))
      (Utilities|Set|Add (LocalVariables|GetL_VisitedTiles) (Utilities|Struct|MakeIntVector (Math|Random|RandomIntegerinRange 0 (- (.x _output_get) 1)) (Math|Random|RandomIntegerinRange 0 (- (.y _output_get) 1)))))
    (:then_1
      ;[1 1 1] Get a random element from the visited list
      (Utilities|FlowControl|Sequence
        (:then_0
          (bind _result_3 (Utilities|Set|ToArray (LocalVariables|GetL_VisitedTiles)))
          (LocalVariables|SetL_SelectedTile (Utilities|Array|Get(acopy) _result_3 (Math|Random|RandomIntegerinRange 0 (- (Utilities|Array|Length _result_3) 0)))))))
    (:then_2
      ;[1 1 1] Returns the generated map
      (return (LocalVariables|GetL_Map)))))

(fn GenerateRandomTile
  (params (Position :type Int%20Vector%20Structure) (Map :type Map%20of%20Int%20Vector%20Structures%20to%20Integers))
  (LocalVariables|SetL_Pos Position)
  (LocalVariables|SetL_Map Map)
  (Utilities|FlowControl|Sequence
    (:then_0
      (if (> (.x (LocalVariables|GetL_Pos)) 1)
        _))
    (:then_1
      (if (< (.x (LocalVariables|GetL_Pos)) (Utilities|Map|Length (LocalVariables|GetL_Map)))
        _))))

(fn AddDoor
  (params (Direction :type DoorDirection%20Enum :default "NewEnumerator0") (TileId :type Integer))
  ;[1 1 1] Adds a door in the requested direction though a bitwise operation
  (switch Utilities|FlowControl|Switch|SwitchonDoorDirection Direction
    (:NewEnumerator0
      (LocalVariables|SetMask 1))
    (:NewEnumerator1
      (LocalVariables|SetMask 2))
    (:NewEnumerator2
      (LocalVariables|SetMask 4))
    (:NewEnumerator3
      (LocalVariables|SetMask 8)))
  (return (Class|KismetMathLibrary|OrIntInt TileId (LocalVariables|GetMask))))

(fn RemoveDoor
  (params (Direction :type DoorDirection%20Enum :default "NewEnumerator0") (TileId :type Integer))
  ;[1 1 1] Removes a door in the requested direction though a bitwise operation
  (switch Utilities|FlowControl|Switch|SwitchonDoorDirection Direction
    (:NewEnumerator0
      (LocalVariables|SetMask 14))
    (:NewEnumerator1
      (LocalVariables|SetMask 13))
    (:NewEnumerator2
      (LocalVariables|SetMask 11))
    (:NewEnumerator3
      (LocalVariables|SetMask 7)))
  (return (Class|KismetMathLibrary|AndIntInt TileId (LocalVariables|GetMask))))

(fn RemoveExternalDoors
  (params (Map :type Map%20of%20Int%20Vector%20Structures%20to%20Integers))
  (bind _output_get (LocalVariables|SetL_Map Map))
  (bind _keys (Utilities|Map|Keys _output_get))
  (for _array_element _keys
    (LocalVariables|SetL_TileCoord _array_element)
    (Utilities|FlowControl|Sequence
      (:then_0
        ;[1 1 1] Close door: North
        (if (== (.x (LocalVariables|GetL_TileCoord)) 0)
          (bind _result (CallFunction|RemoveDoor "NewEnumerator0" (.Value (Utilities|Map|Find (LocalVariables|GetL_Map) (LocalVariables|GetL_TileCoord)))))
          (Utilities|Map|Add (LocalVariables|GetL_Map) (LocalVariables|GetL_TileCoord) _result)))
      (:then_1
        ;[1 1 1] Close door: South
        (bind _result_2 (CallFunction|GetGridSize (LocalVariables|GetL_Map)))
        (if (== (.x (LocalVariables|GetL_TileCoord)) (- (.x _result_2) 1))
          (bind _result_3 (CallFunction|RemoveDoor "NewEnumerator2" (.Value (Utilities|Map|Find (LocalVariables|GetL_Map) (LocalVariables|GetL_TileCoord)))))
          (Utilities|Map|Add (LocalVariables|GetL_Map) (LocalVariables|GetL_TileCoord) _result_3)))
      (:then_2
        ;[1 1 1] Close door: North
        (if (== (.y (LocalVariables|GetL_TileCoord)) 0)
          (bind _result_4 (CallFunction|RemoveDoor "NewEnumerator3" (.Value (Utilities|Map|Find (LocalVariables|GetL_Map) (LocalVariables|GetL_TileCoord)))))
          (Utilities|Map|Add (LocalVariables|GetL_Map) (LocalVariables|GetL_TileCoord) _result_4)))
      (:then_3
        ;[1 1 1] Close door: South
        (bind _result_5 (CallFunction|GetGridSize (LocalVariables|GetL_Map)))
        (if (== (.y (LocalVariables|GetL_TileCoord)) (- (.y _result_5) 1))
          (bind _result_6 (CallFunction|RemoveDoor "NewEnumerator1" (.Value (Utilities|Map|Find (LocalVariables|GetL_Map) (LocalVariables|GetL_TileCoord)))))
          (Utilities|Map|Add (LocalVariables|GetL_Map) (LocalVariables|GetL_TileCoord) _result_6)))))
  ;[1 1 1] Return closed map
  (return (LocalVariables|GetL_Map)))

(fn GetGridSize
  (params (Map :type Map%20of%20Int%20Vector%20Structures%20to%20Integers))
  (bind _keys (Utilities|Map|Keys Map))
  (for _array_element _keys
    ;[1 1 1] Checks the size by comparing the coordinates
    (if (> (.X (Utilities|Struct|BreakIntVector _array_element)) (LocalVariables|GetL_Rows))
      (LocalVariables|SetL_Rows (.X (Utilities|Struct|BreakIntVector _array_element))))
    (if (> (.Y (Utilities|Struct|BreakIntVector _array_element)) (LocalVariables|GetL_Cols))
      (LocalVariables|SetL_Cols (.Y (Utilities|Struct|BreakIntVector _array_element)))))
  ;[1 1 1] Returns the result
  (return (Utilities|Struct|MakeIntVector (+ (LocalVariables|GetL_Rows) 1) (+ (LocalVariables|GetL_Cols) 1))))

(fn ProcessPerfectLabirynthTile)